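; BP_raton is a 2D mouse NPC that patrols back and forth and damages the player character on overlap.
; Each Tick, MoverRaton uses CantMovimiento as an eight-second timer, toggling Vuelve to reverse direction and mirroring the flipbook by negative X scale.
; Movement is a fixed, unswept local offset per frame, so speed depends on frame rate.
; Ending an overlap draws a debug circle around the other actor.
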(event `self.ReceiveTick`
  (params (DeltaSeconds :type "Float (single-precision)"))
  (`self.moverRaton` DeltaSeconds))

(event `self.ReceiveActorBeginOverlap`
  (params (OtherActor :type "Actor Object Reference"))
  (bind _asbp_character (cast `/Game/2D/Character/BP_Character` OtherActor))
  (`/Game/2D/Character/BP_Character.Recibe Daño` _asbp_character))

(event `self.ReceiveActorEndOverlap`
  (params (OtherActor :type "Actor Object Reference"))
  (`KismetSystemLibrary.DrawDebugCircle` (`self.K2_GetActorLocation` OtherActor) 500.0 12 (struct :`R` 1.0 :`B` 0.088224 :`A` 0.512) 0.5 10.0))

(fn `moverRaton`
  (params (A :type "Float (double-precision)"))
  (if (`self.vuelve`)
    (bind _output_get (set `self.Cant Movimiento` (- (`self.Cant Movimiento`) A)))
    (if (< _output_get 0.0)
      (set `self.vuelve` false)
      (else
        (`self.K2_AddActorLocalOffset` (-55.0 0.0 0.0))
        (`SceneComponent.K2_SetRelativeTransform` (`self.PaperFlipbook`) (`KismetMathLibrary.MakeTransform` (0.0 0.0 0.0) (struct) (-1.0 1.0 1.0)) false false)))
    (else
      (bind _output_get_2 (set `self.Cant Movimiento` (+ A (`self.Cant Movimiento`))))
      (if (> _output_get_2 8.0)
        (set `self.vuelve` true)
        (else
          (`self.K2_AddActorLocalOffset` (55.0 0.0 0.0))
          (`SceneComponent.K2_SetRelativeTransform` (`self.PaperFlipbook`) (`KismetMathLibrary.MakeTransform` (0.0 0.0 0.0)) false false))))))

(fn `UserConstructionScript`)