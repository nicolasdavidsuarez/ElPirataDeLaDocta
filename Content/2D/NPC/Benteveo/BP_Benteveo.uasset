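; BP_Benteveo is a 2D flying bird enemy that dive-attacks the pirate and damages any BP_Character it overlaps via RecibeDaño.
; Ataca stores a target position and picks the horizontal direction.
; Tick then moves the bird toward that fixed point, setting the flipbook's facing.
; After passing the point it climbs away along that direction until a Delay ends the attack and plays a sound; GetEstaAtacando exposes the attack state.
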(event `self.ReceiveActorBeginOverlap`
  (params (OtherActor :type "Actor Object Reference"))
  (bind _asbp_character (cast `/Game/2D/Character/BP_Character` OtherActor))
  (`/Game/2D/Character/BP_Character.Recibe Daño` _asbp_character))

(event `self.ReceiveTick`
  (params (DeltaSeconds :type "Float (single-precision)"))
  (bind _returnvalue_x (`KismetMathLibrary.BreakVector` (`self.K2_GetActorLocation`)))
  (bind (_returnvalue_x_2 _returnvalue_y _returnvalue_z) (`KismetMathLibrary.BreakVector` (`self.K2_GetActorLocation`)))
  (bind _returnvalue_x_3 (`KismetMathLibrary.BreakVector` (`self.K2_GetActorLocation`)))
  (bind (_returnvalue_x_4 _returnvalue_y_2 _returnvalue_z_2) (`KismetMathLibrary.BreakVector` (`self.K2_GetActorLocation`)))
  (bind (_vectorposicionpirata_x _vectorposicionpirata_y _vectorposicionpirata_z) (`KismetMathLibrary.BreakVector` (`self.vectorPosicionPirata`)))
  (bind (_vectorposicionpirata_x_2 _vectorposicionpirata_y_2 _vectorposicionpirata_z_2) (`KismetMathLibrary.BreakVector` (`self.vectorPosicionPirata`)))
  (if (`self.estaAtacando`)
    ;[1 1 1] ataca izquierda a derecha
    (if (`self.deIzquierdaADerecha`)
      (if (`self.pasoObjetivo`)
        (`self.K2_AddActorLocalOffset` (`KismetMathLibrary.MakeVector` (* DeltaSeconds 4500.0) 0.0 (* DeltaSeconds 2000.0)))
        (`KismetSystemLibrary.Delay` 4.0)
        (set `self.estaAtacando` false)
        (set `self.pasoObjetivo` false)
        (`GameplayStatics.PlaySound2D` "/Game/2D/Escenarios/Sonidos/benteveoEdit.benteveoEdit" 1.0 1.0 0.0 null null)
        (elif (and (>= _vectorposicionpirata_x_2 _returnvalue_x_3) (<= _vectorposicionpirata_z_2 _returnvalue_z_2))
          (`self.K2_AddActorLocalOffset` (* (`KismetMathLibrary.Normal` (- (`self.vectorPosicionPirata`) (`self.K2_GetActorLocation`))) (* (`self.velocidaAtaque`) DeltaSeconds)))
          (`SceneComponent.K2_SetRelativeTransform` (`self.PaperFlipbook`) (`KismetMathLibrary.MakeTransform` (0.0 0.0 0.0)) false false)
          (else
            (set `self.pasoObjetivo` true))))
      (elif (`self.pasoObjetivo`)
        (`self.K2_AddActorLocalOffset` (`KismetMathLibrary.MakeVector` (* DeltaSeconds -4500.0) 0.0 (* DeltaSeconds 2000.0)))
        (`KismetSystemLibrary.Delay` 4.0)
        (set `self.estaAtacando` false)
        (set `self.pasoObjetivo` false)
        (`GameplayStatics.PlaySound2D` "/Game/2D/Escenarios/Sonidos/benteveoEdit.benteveoEdit" 1.0 1.0 0.0 null null)
        (elif (and (< _vectorposicionpirata_x _returnvalue_x) (<= _vectorposicionpirata_z _returnvalue_z))
          (`self.K2_AddActorLocalOffset` (* (`KismetMathLibrary.Normal` (- (`self.vectorPosicionPirata`) (`self.K2_GetActorLocation`))) (* DeltaSeconds (`self.velocidaAtaque`))))
          (`SceneComponent.K2_SetRelativeTransform` (`self.PaperFlipbook`) (`KismetMathLibrary.MakeTransform` (0.0 0.0 0.0) (struct) (-1.0 1.0 1.0)) false false)
          (else
            (set `self.pasoObjetivo` true)))))))

(event `self.ReceiveActorEndOverlap`
  (params (OtherActor :type "Actor Object Reference")))

(fn `Ataca`
  (params (dondeAtaca :type "Vector Structure"))
  (locals (NewLocalVar :type "Vector Structure" :default (0.0 0.0 0.0)))
  (bind _returnvalue_x (`KismetMathLibrary.BreakVector` (`self.K2_GetActorLocation`)))
  (bind _output_get (set `self.vectorPosicionPirata` dondeAtaca))
  (set `self.estaAtacando` true)
  (bind _output_get_2 (set `self.vectorPosicionPirata` _output_get))
  (set `self.deIzquierdaADerecha` (> (.x _output_get_2) _returnvalue_x)))

(fn `getEstaAtacando`
  (returns (estaAtacando :type Boolean))
  (return (`self.estaAtacando`)))

(fn `UserConstructionScript`)