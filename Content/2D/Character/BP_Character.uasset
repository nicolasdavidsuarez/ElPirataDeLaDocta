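; 2D character Blueprint that moves along the world X axis and jumps through Enhanced Input.
; BeginPlay adds the IMC_MC mapping context to the player controller's input subsystem.
; Movement input also flips control rotation yaw to face travel direction, based on the sign of X acceleration.
; Tick prints vertical velocity on screen as a debug readout.
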(event `self.ReceiveTick`
  (params (DeltaSeconds :type "Float (single-precision)"))
  (bind (_returnvalue_x _returnvalue_y _returnvalue_z) (`KismetMathLibrary.BreakVector` (`self.GetVelocity`)))
  (`KismetSystemLibrary.PrintString` (`KismetStringLibrary.Conv_DoubleToString` _returnvalue_z) true true (struct :`R` 0.025668 :`G` 0.106054 :`B` 1.0 :`A` 1.0) 2.0 "1"))

(event `self.ReceiveBeginPlay`
  (bind _asplayer_controller (cast `PlayerController` (`self.GetController`)))
  (message `EnhancedInputSubsystemInterface.AddMappingContext` (pcsubsystem `EnhancedInputLocalPlayerSubsystem` _asplayer_controller) "/Game/2D/Character/Inputs/Mapping/IMC_MC.IMC_MC" 0 (struct)))

(event `EnhancedInput|/Game/2D/Character/Inputs/IA_Movimiento`
  (params (ActionValue :type "Float (double-precision)") (ElapsedSeconds :type "Float (double-precision)") (TriggeredSeconds :type "Float (double-precision)") (InputAction :type "InputAction Object Reference" :default "/Game/2D/Character/Inputs/IA_Movimiento.IA_Movimiento"))
  (bind _returnvalue_x (`KismetMathLibrary.BreakVector` (`CharacterMovementComponent.GetCurrentAcceleration` (`self.CharacterMovement`))))
  (:`Triggered`
    (`self.AddMovementInput` (1.0 0.0 0.0) ActionValue)
    (`/Engine/EditorBlueprintResources/StandardMacros.CompareFloat` _returnvalue_x
      (:`>`
        (`Controller.SetControlRotation` (`self.GetController`) (`KismetMathLibrary.MakeRotator` 0.0)))
      (:`<`
        (`Controller.SetControlRotation` (`self.GetController`) (`KismetMathLibrary.MakeRotator` 0.0 0.0 180.0))))))

(event `EnhancedInput|/Game/2D/Character/Inputs/IA_Saltar`
  (params (ActionValue :type Boolean) (ElapsedSeconds :type "Float (double-precision)") (TriggeredSeconds :type "Float (double-precision)") (InputAction :type "InputAction Object Reference" :default "/Game/2D/Character/Inputs/IA_Saltar.IA_Saltar"))
  (:`Triggered`
    (`self.Jump`)))

(fn `UserConstructionScript`)