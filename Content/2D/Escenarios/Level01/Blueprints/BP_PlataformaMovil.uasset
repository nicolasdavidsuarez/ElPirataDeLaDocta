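; BP_PlataformaMovil is a 2D level platform that shuttles back and forth along its local X axis.
; Tick passes delta time to MoverPlataforma, which offsets the actor at a constant speed independent of frame rate.
; An elapsed-time counter counts up and down between zero and a hardcoded limit, flipping the Vuelve direction flag at each end.
; The frame that flips direction applies no movement.
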(event `self.ReceiveTick`
  (params (DeltaSeconds :type "Float (single-precision)"))
  (`self.moverPlataforma` DeltaSeconds))

(fn `moverPlataforma`
  (params (A :type "Float (double-precision)"))
  (if (`self.vuelve`)
    (bind _output_get (set `self.cantMovimiento` (- (`self.cantMovimiento`) A)))
    (if (< _output_get 0.0)
      (set `self.vuelve` false)
      (else
        (`self.K2_AddActorLocalOffset` (`KismetMathLibrary.MakeVector` (* A -1000.0)))))
    (else
      (bind _output_get_2 (set `self.cantMovimiento` (+ A (`self.cantMovimiento`))))
      (if (> _output_get_2 5.0)
        (set `self.vuelve` true)
        (else
          (`self.K2_AddActorLocalOffset` (`KismetMathLibrary.MakeVector` (* A 1000.0))))))))

(fn `UserConstructionScript`)