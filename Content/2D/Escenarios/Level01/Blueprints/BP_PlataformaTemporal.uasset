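; BP_PlataformaTemporal is a temporary 2D Paper sprite platform that disappears after being hit and later returns.
; A component hit sets SeDesvanece, making Tick run EfectoDesvanecer, which flickers tint and alpha, alongside BorrarPlataforma's countdown.
; When that countdown expires, the platform turns nearly transparent and loses collision.
; ReAparece then restores color and collision after a shorter delay, using Tick-accumulated timers and boolean flags throughout.
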(event `self.ReceiveActorBeginOverlap`
  (params (OtherActor :type "Actor Object Reference")))

(event `self.PaperSprite.OnComponentHit`
  (params (HitComponent :type "PrimitiveComponent Object Reference") (OtherActor :type "Actor Object Reference") (OtherComp :type "PrimitiveComponent Object Reference") (NormalImpulse :type "Vector Structure") (Hit :type "HitResult Structure (by ref)"))
  (set `self.seDesvanece` true))

(event `self.ReceiveTick`
  (params (DeltaSeconds :type "Float (single-precision)"))
  (if (`self.seDesvanece`)
    (`self.efectoDesvanecer` DeltaSeconds)
    (`self.borrarPlataforma` DeltaSeconds)
    (else
      (`self.reAparece` DeltaSeconds))))

(fn `borrarPlataforma`
  (params (A :type "Float (double-precision)"))
  (bind _papersprite (`self.PaperSprite`))
  (bind _returnvalue (+ A (`self.tiempoBorrado`)))
  (set `self.tiempoBorrado` _returnvalue)
  (if (> _returnvalue 3.0)
    (`PrimitiveComponent.SetCollisionEnabled` _papersprite "NoCollision")
    (`PaperSpriteComponent.SetSpriteColor` _papersprite (struct :`A` 0.1))
    (set `self.seDesvanece` false)
    (set `self.tiempoBorrado` 0.0)
    (set `self.debeAparecer` true)))

(fn `efectoDesvanecer`
  (params (A :type "Float (double-precision)"))
  (bind _output_get (set `self.aceleracionLuces` (+ A (`self.aceleracionLuces`))))
  (if (`self.cambioColor`)
    (bind _output_get_2 (set `self.tiempo` (- (`self.tiempo`) A)))
    (if (< _output_get_2 0.0)
      (set `self.cambioColor` false)
      (set `self.aceleracionLuces` 0.0)
      (else
        (bind _returnvalue (- 1.0 _output_get))
        (`PaperSpriteComponent.SetSpriteColor` (`self.PaperSprite`) (make `LinearColor` 0.9 1.0 0.9 _returnvalue))))
    (else
      (bind _output_get_3 (set `self.tiempo` (+ A (`self.tiempo`))))
      (if (> _output_get_3 0.3)
        (set `self.cambioColor` true)
        (set `self.aceleracionLuces` 0.0)
        (else
          (`PaperSpriteComponent.SetSpriteColor` (`self.PaperSprite`) (make `LinearColor` 1.0 0.8 0.8 _returnvalue)))))))

(fn `reAparece`
  (params (A :type "Float (double-precision)"))
  (bind _papersprite (`self.PaperSprite`))
  (if (`self.debeAparecer`)
    (bind _output_get (set `self.tiempoReaparicion` (+ A (`self.tiempoReaparicion`))))
    (if (> _output_get 2.0)
      (`PaperSpriteComponent.SetSpriteColor` _papersprite (struct :`R` 1.0 :`G` 1.0 :`B` 1.0 :`A` 1.0))
      (`PrimitiveComponent.SetCollisionEnabled` _papersprite "QueryAndPhysics")
      (set `self.seDesvanece` false)
      (set `self.tiempoReaparicion` 0.0)
      (set `self.debeAparecer` false))))

(fn `UserConstructionScript`)