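; Shadow actor for the Level01 parallax background that sways back and forth along a curved path.
; Tick passes delta seconds to MovimientoSombras, which ramps VariacionSombra up and down between roughly 0 and 3, flipping SombraSube at each limit.
; That value sets opposing, complementary local X and Z offsets, reversed on the way down.
; Offsets apply per frame without delta scaling, so travel depends on frame rate.
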(event `self.ReceiveTick`
  (params (DeltaSeconds :type "Float (single-precision)"))
  (`self.MovimientoSombras` DeltaSeconds))

(fn `MovimientoSombras`
  (params (A :type "Float (double-precision)"))
  (bind _variacionsombra (`self.variacionSombra`))
  (bind _variacionsombra_2 (`self.variacionSombra`))
  (bind _variacionsombra_3 (`self.variacionSombra`))
  (bind _variacionsombra_4 (`self.variacionSombra`))
  (bind _variacionsombra_5 (`self.variacionSombra`))
  (if (`self.sombraSube`)
    (set `self.variacionSombra` (+ A _variacionsombra_2))
    (else
      (set `self.variacionSombra` (- _variacionsombra_2 A))))
  (if (`self.sombraSube`)
    (`self.K2_AddActorLocalOffset` (`KismetMathLibrary.MakeVector` _variacionsombra_5 0.0 (* (- 3.0 _variacionsombra_5) -1.0)))
    (if (> _variacionsombra_4 3.0)
      (set `self.sombraSube` false)
      (elif (< _variacionsombra_4 0.0)
        (set `self.sombraSube` true)))
    (else
      (`self.K2_AddActorLocalOffset` (`KismetMathLibrary.MakeVector` (* _variacionsombra_3 -1.0) 0.0 (- 3.0 _variacionsombra_3)))
      (if (> _variacionsombra 3.0)
        (set `self.sombraSube` false)
        (elif (< _variacionsombra 0.0)
          (set `self.sombraSube` true))))))

(fn `UserConstructionScript`)